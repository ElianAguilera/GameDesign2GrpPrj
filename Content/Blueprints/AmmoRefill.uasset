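; Ammo refill pickup that stockpiles ammo over time for the player's BananaGun.
; A looping delay from BeginPlay increments ReadyAmmo every few seconds with no upper limit.
; When BP_ThirdPersonCharacter overlaps GetAmmoHitbox, it passes the stock to the BananaGun found by GetActorOfClass, resets it and plays a sound at world origin.
; ChangeWeapon is an empty stub.
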(event `self.ReceiveBeginPlay`
  ; Creates ammo for player to collect [ADD LIMITS]
  (`KismetSystemLibrary.Delay` 5.0 :!label _label)
  (`/Engine/EditorBlueprintResources/StandardMacros.IncrementFloat` (`self.ReadyAmmo`)
    (:`  `
      (goto _label))))

(event `self.GetAmmoHitbox.OnComponentBeginOverlap`
  (params (OverlappedComponent :type "PrimitiveComponent Object Reference") (OtherActor :type "Actor Object Reference") (OtherComp :type "PrimitiveComponent Object Reference") (OtherBodyIndex :type Integer) (bFromSweep :type Boolean) (SweepResult :type "HitResult Structure (by ref)"))
  ; Collects ammo when player runs close to it
  (cast `/Game/ThirdPerson/Blueprints/BP_ThirdPersonCharacter` OtherActor)
  (bind _returnvalue (`GameplayStatics.GetActorOfClass` "/Game/Blueprints/BananaGun.BananaGun_C"))
  (`/Game/Blueprints/BPIs/BPI_Weapons.WeaponAddAmmo` _returnvalue (`self.ReadyAmmo`))
  (set `self.ReadyAmmo` 0.0)
  (`GameplayStatics.PlaySoundAtLocation` "/Game/Sound/power-up-type-1-230548_Cue.power-up-type-1-230548_Cue" (0.0 0.0 0.0) (struct) 1.0 1.0 0.0 null null null null))

(fn `ChangeWeapon`
  (returns (WeaponMesh :type "SkeletalMeshComponent Object Reference"))
  (return null))

(fn `UserConstructionScript`)