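; BananaGun is a weapon Blueprint that fires BananaBullet actors.
; UseWeapon spawns a bullet at the BulletDirection component's transform, then blocks firing for one second through an IsFireable flag and a Delay.
; WeaponAddAmmo increases an Ammo count, but firing neither checks nor spends it.
; ChangeWeapon is an empty stub.
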(event `/Game/Blueprints/BPIs/BPI_Weapons.UseWeapon`
  (bind (_returnvalue_location _returnvalue_rotation) (`KismetMathLibrary.BreakTransform` (`SceneComponent.K2_GetComponentToWorld` (`self.BulletDirection`))))
  ; Uses Weapon
  (if (`self.IsFireable`)
    (`|SpawnActorFromClass` "/Game/Blueprints/BananaBullet.BananaBullet_C" (`KismetMathLibrary.MakeTransform` _returnvalue_location _returnvalue_rotation) "Undefined" "MultiplyWithRoot" null null)
    (set `self.IsFireable` false)
    (`KismetSystemLibrary.Delay` 1.0)
    (set `self.IsFireable` true)))

(event `/Game/Blueprints/BPIs/BPI_Weapons.WeaponAddAmmo`
  (params (AddAmmo :type "Float (double-precision)"))
  ; adds ammo
  (set `self.Ammo` (+ AddAmmo (`self.Ammo`))))

(fn `ChangeWeapon`
  (returns (WeaponMesh :type "SkeletalMeshComponent Object Reference"))
  (return null))

(fn `UserConstructionScript`)