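; Enemy1 is a melee enemy character that chases the player and scales its health and speed by round.
; Every Tick it turns toward the player, reissues AIMoveTo and deals damage while the player overlaps E1Hitbox and is not invulnerable.
; BeginPlay randomizes walk speed slightly above Speed.
; DamageEnemy reduces health and, below one, destroys the actor and decrements AiSpawner's remaining-enemy count.
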(event `self.ReceiveBeginPlay`
  (bind _speed (`self.Speed`))
  ; Sets max speed
  (set `CharacterMovementComponent.MaxWalkSpeed` (`KismetMathLibrary.RandomFloatInRange` _speed (+ _speed 50.0)) (`self.CharacterMovement`)))

(event `self.ReceiveTick`
  (params (DeltaSeconds :type "Float (single-precision)"))
  ; AI Movement
  (`self.LookAtPlayer`)
  (`|AIMoveTo` self (0.0 0.0 0.0) (`GameplayStatics.GetPlayerCharacter` 0) 0.0 true
    (:`then`
      ; Player Damage Check
      (bind _asbp_third_person_character (cast `/Game/ThirdPerson/Blueprints/BP_ThirdPersonCharacter` (`GameplayStatics.GetPlayerCharacter` 0)))
      (if (`/Game/ThirdPerson/Blueprints/BP_ThirdPersonCharacter.Invulnerable` _asbp_third_person_character)
        _
        (elif (`self.InE1`)
          (`GameplayStatics.ApplyDamage` (`GameplayStatics.GetPlayerCharacter` 0) 1.0))))))

(event `self.E1Hitbox.OnComponentBeginOverlap`
  (params (OverlappedComponent :type "PrimitiveComponent Object Reference") (OtherActor :type "Actor Object Reference") (OtherComp :type "PrimitiveComponent Object Reference") (OtherBodyIndex :type Integer) (bFromSweep :type Boolean) (SweepResult :type "HitResult Structure (by ref)"))
  ; Checks if player is inside Enemy hitbox
  (cast `/Game/ThirdPerson/Blueprints/BP_ThirdPersonCharacter` OtherActor)
  (set `self.InE1` true))

(event `self.E1Hitbox.OnComponentEndOverlap`
  (params (OverlappedComponent :type "PrimitiveComponent Object Reference") (OtherActor :type "Actor Object Reference") (OtherComp :type "PrimitiveComponent Object Reference") (OtherBodyIndex :type Integer))
  ; Checks if player is inside Enemy hitbox
  (cast `/Game/ThirdPerson/Blueprints/BP_ThirdPersonCharacter` OtherActor)
  (set `self.InE1` false))

(event `/Game/Blueprints/BPIs/BPI_DamageEnemies.DamageEnemy`
  (params (Damage :type "Float (double-precision)"))
  (bind _output_get (set `self.E1Health` (- (`self.E1Health`) Damage)))
  (if (>= _output_get 1.0)
    (`KismetSystemLibrary.PrintString` "Hello")
    (else
      (`self.K2_DestroyActor`)
      (bind _returnvalue (`GameplayStatics.GetActorOfClass` "/Game/Blueprints/AiSpawner.AiSpawner_C"))
      (bind _result (`/Engine/EditorBlueprintResources/StandardMacros.DecrementFloat` (`/Game/Blueprints/AiSpawner.ERemaining` _returnvalue))
        (:`  `
          (bind _output_get_2 (set `/Game/Blueprints/AiSpawner.ERemaining` _result _returnvalue))
          (if (<= _output_get_2 0.0)
            _))))))

(event `/Game/Blueprints/BPIs/BPI_Scaling.EnemyScaling`
  (params (EnemyRoundScaling :type "Float (double-precision)"))
  ; Enemy Stat Scaling
  (set `self.E1Health` (* (+ EnemyRoundScaling (`self.E1Health`)) 1.1))
  (set `self.Speed` (+ EnemyRoundScaling 250.0)))

(fn `LookAtPlayer`
  (bind (_returnvalue_roll _returnvalue_pitch _returnvalue_yaw) (`KismetMathLibrary.BreakRotator` (`KismetMathLibrary.FindLookAtRotation` (`self.K2_GetActorLocation`) (`self.K2_GetActorLocation` (`GameplayStatics.GetPlayerCharacter` 0)))))
  ; looks at player (unused)
  (`self.K2_SetActorRotation` (`KismetMathLibrary.MakeRotator` _returnvalue_roll 0.0 _returnvalue_yaw)))

(fn `UserConstructionScript`)